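; GameInstance Blueprint that saves and restores the player character's location through a SaveGame_BP object and a single "Guardado" slot.
; Save records the location in the SaveGame object, creating it if needed, but writes to the slot only when it has just created the object.
; Load checks that the slot exists, caches the loaded object and moves the player character to the stored position by teleport.
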(event Custom|Save
  ;[0.141 0.2712 1] Save
  (Utilities|IsValid (Variables|Default|GetSaveGame)
    (:Is%20Valid
      (Variables|/Game/MyContent/01_Levels/SavingData/SaveGame_BP.SaveGame_BP_C|SetPlayerPos (Variables|Default|GetSaveGame) (Transformation|GetActorLocation (Game|GetPlayerCharacter 0))))
    (:Is%20Not%20Valid
      (bind _returnvalue (SaveGame|CreateSaveGameObject "/Game/MyContent/01_Levels/SavingData/SaveGame_BP.SaveGame_BP_C"))
      (bind _output_get (Variables|Default|SetSaveGame _returnvalue))
      (Variables|/Game/MyContent/01_Levels/SavingData/SaveGame_BP.SaveGame_BP_C|SetPlayerPos _output_get (Transformation|GetActorLocation (Game|GetPlayerCharacter 0)))
      (SaveGame|SaveGametoSlot (Variables|Default|GetSaveGame) "Guardado"))))

(event Custom|Load
  ;[1 0.2249 0.8555] Load
  (bind _returnvalue (SaveGame|DoesSaveGameExist "Guardado"))
  (if _returnvalue
    (bind _returnvalue_2 (SaveGame|LoadGamefromSlot "Guardado"))
    (bind _assave_game_bp (Utilities|Casting|CastToSaveGame_BP _returnvalue_2))
    (bind _output_get (Variables|Default|SetSaveGame _assave_game_bp))
    (Transformation|SetActorLocation (Game|GetPlayerCharacter 0) (Variables|/Game/MyContent/01_Levels/SavingData/SaveGame_BP.SaveGame_BP_C|GetPlayerPos _output_get) false true)))
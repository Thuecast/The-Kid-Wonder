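; Health pickup actor that heals the Luke player character on overlap.
; On BeginPlay it applies its HealtSprite to a Paper2D sprite component.
; An overlapping LukeCharacter_BP receives HealPlayer with the Health amount, and a heal sound plays at the pickup's location.
; A Sequence node then destroys the pickup, even when the overlapping actor fails the character cast.
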(event EventBeginPlay
  (Rendering|Components|Sprite|SetSprite (Variables|Default|GetPaperSprite) (Variables|Default|GetHealtSprite)))

(event Collision|EventActorBeginOverlap
  (params (OtherActor :type Actor%20Object%20Reference))
  (Utilities|FlowControl|Sequence
    (:then_0
      (bind _asluke_character_bp (Utilities|Casting|CastToLukeCharacter_BP OtherActor))
      (Default|HealPlayer _asluke_character_bp (Variables|Default|GetHealth))
      (Audio|PlaySoundatLocation "/Game/MyContent/04_SFX/Buffs_Heals_SFX/02_Heal_02.02_Heal_02" (Transformation|GetActorLocation) "0, 0, 0" 1.0 1.0 0.0 0 0 0 0))
    (:then_1
      (Actor|DestroyActor))))

(event EventTick
  (params (DeltaSeconds :type Float%20%28single-precision%29)))

(fn ConstructionScript)
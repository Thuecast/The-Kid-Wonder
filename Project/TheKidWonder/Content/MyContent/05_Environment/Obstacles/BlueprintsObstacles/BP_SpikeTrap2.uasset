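; Spike trap obstacle that stays hidden from game start until something overlaps its Box, then damages the player.
; Any overlap reveals the trap permanently, but only LukeCharacter_BP takes Damage and triggers a Paper flipbook component added at runtime.
; The flipbook stops after a 0.2-second delay and is destroyed when the character leaves the box, while the actor itself stays visible.
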(event OnComponentBeginOverlap(Box)
  (params (OverlappedComponent :type Primitive%20Component%20Object%20Reference) (OtherActor :type Actor%20Object%20Reference) (OtherComp :type Primitive%20Component%20Object%20Reference) (OtherBodyIndex :type Integer) (bFromSweep :type Boolean) (SweepResult :type Hit%20Result%20Structure%20%28by%20ref%29))
  (Rendering|SetActorHiddenInGame false)
  (bind _asluke_character_bp (Utilities|Casting|CastToLukeCharacter_BP OtherActor))
  (bind _returnvalue (AddComponent|AddPaperFlipbookComponent false))
  (Game|Damage|ApplyDamage _asluke_character_bp (Variables|Default|GetDamage) 0 0)
  (Utilities|FlowControl|Delay 0.2)
  (Audio|Components|Audio|Stop _returnvalue))

(event OnComponentEndOverlap(Box)
  (params (OverlappedComponent :type Primitive%20Component%20Object%20Reference) (OtherActor :type Actor%20Object%20Reference) (OtherComp :type Primitive%20Component%20Object%20Reference) (OtherBodyIndex :type Integer))
  (Utilities|Casting|CastToLukeCharacter_BP OtherActor)
  (Components|DestroyComponent (stale OnComponentBeginOverlap(Box) _returnvalue)))

(event EventBeginPlay
  (Rendering|SetActorHiddenInGame true))

(event Collision|EventActorBeginOverlap
  (params (OtherActor :type Actor%20Object%20Reference)))

(event EventTick
  (params (DeltaSeconds :type Float%20%28single-precision%29)))

(fn ConstructionScript)
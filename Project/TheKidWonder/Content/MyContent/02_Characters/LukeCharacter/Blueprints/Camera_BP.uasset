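; Orthographic side-view camera actor that follows the player character while keeping its view inside the level's bounds.
; Each Tick it finds the Main_Level_TM actor, moves to the player's position, and clamps X and Z to limits from GetLimitX and GetLimitZ.
; Those helpers inset the map actor's bounds by half the view size, derived from OrthoWidth and AspectRatio, while Y follows the player unclamped.
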(event EventBeginPlay)

(event Collision|EventActorBeginOverlap
  (params (OtherActor :type Actor%20Object%20Reference)))

(event EventTick
  (params (DeltaSeconds :type Float%20%28single-precision%29))
  (bind _returnvalue (Game|GetPlayerCharacter 0))
  (bind _returnvalue_2 (Transformation|GetActorLocation _returnvalue))
  (bind _returnvalue_3 (Actor|GetActorOfClass "/Game/MyContent/05_Environment/LevelBuild/OakForest/2Paper_Convert/Sprites/TileSetMap/Main_Level_TM.Main_Level_TM_C"))
  (Transformation|SetActorLocation (Math|Vector|MakeVector (Math|Float|Clamp(Float) (.x _returnvalue_2) (.LimitXMin (CallFunction|GetLimitX _returnvalue_3)) (.LimitXMax (CallFunction|GetLimitX _returnvalue_3))) (.y _returnvalue_2) (Math|Float|Clamp(Float) (.z _returnvalue_2) (.LimitZMin (CallFunction|GetLimitZ _returnvalue_3)) (.LimitZMax (CallFunction|GetLimitZ _returnvalue_3)))) false false))

(fn ConstructionScript)

(fn GetLimitZ
  (params (MapActor :type Actor%20Object%20Reference))
  (bind (_origin _boxextent) (Collision|GetActorBounds MapActor false true))
  (bind _cameracomponent (Variables|CameraActor|GetCameraComponent))
  (bind _orthowidth (Variables|/Script/Engine.CameraComponent|GetOrthoWidth _cameracomponent))
  (bind _aspectratio (Variables|/Script/Engine.CameraComponent|GetAspectRatio _cameracomponent))
  (bind _returnvalue (/ _orthowidth _aspectratio))
  (bind _returnvalue_2 (/ _returnvalue 2.0))
  (return (- (+ (.z _origin) (.z _boxextent)) _returnvalue_2) (+ (- (.z _origin) (.z _boxextent)) _returnvalue_2)))

(fn GetLimitX
  (params (MapActor :type Actor%20Object%20Reference))
  (bind (_origin _boxextent) (Collision|GetActorBounds MapActor false true))
  (bind _cameracomponent (Variables|CameraActor|GetCameraComponent))
  (bind _orthowidth (Variables|/Script/Engine.CameraComponent|GetOrthoWidth _cameracomponent))
  (bind _returnvalue (/ _orthowidth 2.0))
  (return (- (+ (.x _origin) (.x _boxextent)) _returnvalue) (+ (- (.x _origin) (.x _boxextent)) _returnvalue)))
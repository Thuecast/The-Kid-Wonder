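; Flying bat enemy for a 2D flipbook game that patrols, shoots at the player and dies from damage.
; Tick moves it along X with a Timeline-driven vertical bob, flipping direction through distance checks from its spawn point.
; A sphere trace plus an eye line trace detects LukeCharacter_BP, pausing patrol to face the player and fire BatBullet_BP after a delay.
; AnyDamage reduces life; death stops movement and destroys the actor after a delay.
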(event Custom|Die
  (Variables|Default|SetEnemyLife 0.0)
  (CallFunction|EnemyDeath)
  (Utilities|FlowControl|Delay 1.5)
  (Actor|DestroyActor)
  (Audio|PlaySoundatLocation "/Game/MyContent/04_SFX/Battle_SFX/69_Enemy_death_01.69_Enemy_death_01" (Transformation|GetActorLocation) "0, 0, 0" 1.0 1.0 0.0 0 0 0 0))

(event EventBeginPlay
  (Variables|Default|SetEnemyLife (Variables|Default|GetEnemyLife))
  (Variables|Default|SetinitPos (Transformation|GetActorLocation))
  (bind _zmovement (Timeline|ZMovement Play)
    (:Update
      (Variables|Default|SetzMove _zmovement))))

(event Game|Damage|EventAnyDamage
  (params (Damage :type Float%20%28single-precision%29) (DamageType :type Damage%20Type%20Object%20Reference) (InstigatedBy :type Controller%20Object%20Reference) (DamageCauser :type Actor%20Object%20Reference))
  (if (> (Math|Float|Clamp(Float) (- (Variables|Default|GetEnemyLife) Damage) 0.0 (Variables|Default|GetEnemyLife)) 0.0)
    (Variables|Default|SetEnemyLife (Math|Float|Clamp(Float) (- (Variables|Default|GetEnemyLife) Damage) 0.0 (Variables|Default|GetEnemyLife)))
    (Utilities|FlowControl|DoOnce false
      (:Completed
        (Sprite|SetFlipbook (Variables|Default|GetSprite) "/Game/MyContent/02_Characters/Enemies/EnemyBat/FB/BatHit_FB.BatHit_FB")
        (Audio|PlaySoundatLocation "/Game/MyContent/04_SFX/Player_Movement_SFX/61_Hit_03.61_Hit_03" (Transformation|GetActorLocation) "0, 0, 0" 1.0 1.0 0.0 0 0 0 0)))
    (else
      (CallFunction|Die))))

(event EventTick
  (params (DeltaSeconds :type Float%20%28single-precision%29))
  (if (> (Variables|Default|GetEnemyLife) 0.0)
    (bind _playerdetected (CallFunction|SingleCheckSphere))
    (if _playerdetected
      (Sprite|SetFlipbook (Variables|Default|GetSprite) "/Game/MyContent/02_Characters/Enemies/EnemyBat/FB/BatFly_FB.BatFly_FB")
      (CallFunction|SetDirectionandRotation)
      (Utilities|FlowControl|Delay 1.5)
      (if (> (Variables|Default|GetEnemyLife) 0.0)
        (CallFunction|EnemyShoot))
      (else
        (CallFunction|EnemyMovement)
        (CallFunction|EnemyPatroll)))
    (else
      (CallFunction|Die))))

(fn ConstructionScript)

(fn SingleCheckSphere
  (bind _capsulecomponent (Variables|Collision|GetCapsuleComponent))
  (bind _returnvalue (Transformation|GetWorldLocation _capsulecomponent))
  (bind (_outhit _returnvalue_2) (Collision|SphereTraceByChannel _returnvalue _returnvalue (Variables|Default|GetDetectionRadius) "TraceTypeQuery3" false 0 "ForOneFrame"))
  (if _returnvalue_2
    (bind _asluke_character_bp (Utilities|Casting|CastToLukeCharacter_BP (.HitActor (Collision|BreakHitResult _outhit))))
    (bind _detected (CallFunction|CheckVision _asluke_character_bp))
    (if _detected
      (return true)
      (else
        (return false)))
    (else
      (return false))))

(fn CheckVision
  (params (playerTarget :type Luke%20Character%20BP%20Object%20Reference))
  (Utilities|IsValid playerTarget
    (:Is%20Valid
      (bind _outhit (Collision|LineTraceByChannel (Transformation|GetWorldLocation (Variables|Default|GetEyes)) (Transformation|GetActorLocation playerTarget) "TraceTypeQuery3" false 0 "ForOneFrame"))
      (Utilities|Casting|CastToLukeCharacter_BP (.HitActor (Collision|BreakHitResult _outhit))
        (:then
          (return true))
        (:CastFailed
          (return false))))))

(fn EnemyDeath
  (bind _sprite (Variables|Default|GetSprite))
  (Sprite|SetFlipbook (Variables|Default|GetSprite) "/Game/MyContent/02_Characters/Enemies/EnemyBat/FB/BatHit_FB.BatHit_FB")
  (Components|Timeline|SetLooping _sprite false)
  (Audio|Components|Audio|Play _sprite)
  (Class|NavMovementComponent|StopActiveMovement (Variables|Character|GetCharacterMovement)))

(fn EnemyMovement
  (bind _returnvalue (Transformation|GetActorLocation))
  (bind _enemydirection (Variables|Default|GetenemyDirection))
  (bind _sprite (Variables|Default|GetSprite))
  (Transformation|SetActorLocation (Math|Vector|MakeVector (+ (* (Utilities|Time|GetWorldDeltaSeconds) (Variables|Default|GetenemySpeed) _enemydirection) (.x _returnvalue)) (.y _returnvalue) (+ (.z (Variables|Default|GetinitPos)) (* (Variables|Default|GetzMove) (Variables|Default|GetverticalDistance)))) false false)
  (Sprite|SetFlipbook _sprite "/Game/MyContent/02_Characters/Enemies/EnemyBat/FB/BatFly_FB.BatFly_FB")
  (Transformation|SetRelativeScale3D _sprite (Math|Vector|MakeVector _enemydirection 1.0 1.0)))

(fn EnemyPatroll
  (Utilities|FlowControl|Sequence
    (:then_0
      (bind _ldetected (CallFunction|LimitRight))
      (if (not _ldetected)
        (bind _output_get (Variables|Default|SetenemyDirection (* (Variables|Default|GetenemyDirection) -1.0)))
        (Transformation|SetRelativeRotation (Variables|Default|GetSprite) (Math|Rotator|MakeRotator _output_get _output_get _output_get) false false)))
    (:then_1
      (bind _ldetected_2 (CallFunction|LimitLeft))
      (if (not _ldetected_2)
        (bind _output_get_2 (Variables|Default|SetenemyDirection (* (Variables|Default|GetenemyDirection) -1.0)))
        (Transformation|SetRelativeRotation (Variables|Default|GetSprite) (Math|Rotator|MakeRotator _output_get_2 _output_get_2 _output_get_2) false false)))))

(fn EnemyShoot
  (bind _eyes (Variables|Default|GetEyes))
  (bind _sprite (Variables|Default|GetSprite))
  (bind _sprite_2 (Variables|Default|GetSprite))
  (bind _returnvalue (Transformation|GetWorldLocation _eyes))
  (if (< (.x (Transformation|GetWorldLocation (Variables|Default|GetEyes))) (.x (Transformation|GetActorLocation (Game|GetPlayerCharacter 0))))
    (bind _returnvalue_2 (Game|SpawnActorfromClass "/Game/MyContent/02_Characters/Enemies/EnemyBat/Bat_BP/BatBullet_BP.BatBullet_BP_C" (Math|Transform|MakeTransform (Transformation|GetWorldLocation (Variables|Default|GetEyes)) "0, 0, 0" "1.000000,1.000000,1.000000") "AlwaysSpawn" "MultiplyWithRoot" 0 (Variables|Default|GetbulletInfo) 3.0 0))
    (Default|SetDirectionandRotation _returnvalue_2)
    (Sprite|SetFlipbook (Variables|Default|GetSprite) "/Game/MyContent/02_Characters/Enemies/EnemyBat/FB/BatAttack_FB.BatAttack_FB")
    (Components|Timeline|SetLooping _sprite_2 true)
    (Audio|Components|Audio|Play _sprite_2)
    (else
      (bind _returnvalue_3 (Game|SpawnActorfromClass "/Game/MyContent/02_Characters/Enemies/EnemyBat/Bat_BP/BatBullet_BP.BatBullet_BP_C" (Math|Transform|MakeTransform (Math|Vector|MakeVector (- (.x _returnvalue) 1e+01) (.y _returnvalue) (.z _returnvalue)) "0, 0, 0" "1.000000,1.000000,1.000000") "AlwaysSpawn" "MultiplyWithRoot" 0 (Variables|Default|GetbulletInfo) 3.0 0))
      (Default|SetDirectionandRotation _returnvalue_3)
      (Sprite|SetFlipbook (Variables|Default|GetSprite) "/Game/MyContent/02_Characters/Enemies/EnemyBat/FB/BatAttack_FB.BatAttack_FB")
      (Components|Timeline|SetLooping _sprite true)
      (Audio|Components|Audio|Play _sprite))))

(fn LimitRight
  (return (>= (.x (Transformation|GetActorLocation)) (+ (.x (Variables|Default|GetinitPos)) (Variables|Default|GetDistance)))))

(fn LimitLeft
  (return (<= (.x (Transformation|GetActorLocation)) (.x (Variables|Default|GetinitPos)))))

(fn SetDirectionandRotation
  (bind _returnvalue (Transformation|GetActorLocation))
  (bind _returnvalue_2 (Game|GetPlayerCharacter 0))
  (bind _returnvalue_3 (Transformation|GetActorLocation _returnvalue_2))
  (bind _returnvalue_4 (Math|Rotator|FindLookatRotation _returnvalue _returnvalue_3))
  (if (>= (Variables|Default|GetenemyDirection) 0.0)
    (Transformation|SetRelativeRotation (Variables|Default|GetSprite) (Math|Rotator|FindLookatRotation (Transformation|GetActorLocation) (Transformation|GetActorLocation (Game|GetPlayerCharacter 0))) false false)
    (else
      (Transformation|SetRelativeRotation (Variables|Default|GetSprite) (Math|Rotator|MakeRotator (- (.roll _returnvalue_4) 1.8e+02) (- (.pitch _returnvalue_4) 1.8e+02) (.yaw _returnvalue_4)) false false))))
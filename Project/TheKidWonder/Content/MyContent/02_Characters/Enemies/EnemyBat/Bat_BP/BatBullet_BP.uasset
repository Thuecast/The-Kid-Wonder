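; BatBullet_BP is the bat enemy's projectile, a flipbook bullet whose sprite, movement type, speed and damage come from BulletType.
; Each tick it moves along BulletDirection without sweep; the Following type first re-aims direction and sprite rotation at the player.
; Any overlap destroys it, damaging the other actor first if it is a Character, and its lifespan otherwise limits how long it lives.
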(event EventBeginPlay
  (Sprite|SetFlipbook (Variables|Default|GetBulletFB) (.bulletsprite (Variables|Default|GetbulletType)))
  (Actor|SetLifeSpan (Variables|Default|GetlifeTime)))

(event EventTick
  (params (DeltaSeconds :type Float%20%28single-precision%29))
  (switch Utilities|FlowControl|Switch|SwitchonBatBullet_Enum (.bullettype (Variables|Default|GetbulletType))
    (:NewEnumerator0
      (CallFunction|BulletMovement))
    (:NewEnumerator1
      (CallFunction|SetDirectionandRotation)
      (CallFunction|BulletMovement))))

(event Collision|EventActorBeginOverlap
  (params (OtherActor :type Actor%20Object%20Reference))
  (Utilities|FlowControl|Sequence
    (:then_0
      (bind _ascharacter (Utilities|Casting|CastToCharacter OtherActor))
      (Game|Damage|ApplyDamage _ascharacter (.bulletdamage (Variables|Default|GetbulletType)) 0 0))
    (:then_1
      (Actor|DestroyActor))))

(fn ConstructionScript)

(fn BulletMovement
  (Transformation|SetActorLocation (+ (* (* (Utilities|Time|GetWorldDeltaSeconds) (.bulletspeed (Variables|Default|GetbulletType))) (Variables|Default|GetbulletDirection)) (Transformation|GetActorLocation)) false false))

(fn SetDirectionandRotation
  (bind _returnvalue (Game|GetPlayerCharacter 0))
  (Variables|Default|SetbulletDirection (Math|Vector|GetUnitDirection(Vector) (Transformation|GetActorLocation) (Transformation|GetActorLocation _returnvalue)))
  (Transformation|SetRelativeRotation (Variables|Default|GetBulletFB) (Math|Rotator|FindLookatRotation (Transformation|GetActorLocation) (Transformation|GetActorLocation _returnvalue)) false false))
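; Base enemy Blueprint, a flipbook-sprite character that takes damage and dies.
; AnyDamage subtracts from MaxLife, which doubles as current health, and plays hit flipbook and sound through a DoOnce with no reset.
; At zero, Die stops movement, disables capsule collision, shows the hit flipbook, then destroys the actor with a death sound after a delay.
; A separate TakeDamage function also lowers health but is not called here.
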(event Custom|Die
  ;[1 1 1] Hit and Die
  (Variables|Default|SetmaxLife 0.0)
  (Sprite|SetFlipbook (Variables|Default|GetSprite) "/Game/MyContent/02_Characters/Enemies/EnemyMonster/Sprites/Monster_FB/MonsterHit_FB.MonsterHit_FB")
  (Components|Movement|StopMovementImmediately (Variables|Character|GetCharacterMovement))
  (Collision|SetCollisionEnabled (Variables|Collision|GetCapsuleComponent) "NoCollision")
  (Utilities|FlowControl|Delay 1.5)
  (Actor|DestroyActor)
  (Audio|PlaySoundatLocation "/Game/MyContent/04_SFX/Battle_SFX/69_Enemy_death_01.69_Enemy_death_01" (Transformation|GetActorLocation) "0, 0, 0" 1.0 1.0 0.0 0 0 0 0))

(event EventBeginPlay
  (Variables|Default|SetmaxLife (Variables|Default|GetmaxLife)))

(event Collision|EventActorBeginOverlap
  (params (OtherActor :type Actor%20Object%20Reference)))

(event EventTick
  (params (DeltaSeconds :type Float%20%28single-precision%29)))

(event Game|Damage|EventAnyDamage
  (params (Damage :type Float%20%28single-precision%29) (DamageType :type Damage%20Type%20Object%20Reference) (InstigatedBy :type Controller%20Object%20Reference) (DamageCauser :type Actor%20Object%20Reference))
  ;[1 1 1] Hit and Die
  (if (> (Math|Float|Clamp(Float) (- (Variables|Default|GetmaxLife) Damage) 0.0 (Variables|Default|GetmaxLife)) 0.0)
    (Variables|Default|SetmaxLife (Math|Float|Clamp(Float) (- (Variables|Default|GetmaxLife) Damage) 0.0 (Variables|Default|GetmaxLife)))
    (Utilities|FlowControl|DoOnce false
      (:Completed
        (Sprite|SetFlipbook (Variables|Default|GetSprite) "/Game/MyContent/02_Characters/Enemies/EnemyMonster/Sprites/Monster_FB/MonsterHit_FB.MonsterHit_FB")
        (Audio|PlaySoundatLocation "/Game/MyContent/04_SFX/Player_Movement_SFX/61_Hit_03.61_Hit_03" (Transformation|GetActorLocation) "0, 0, 0" 1.0 1.0 0.0 0 0 0 0)))
    (else
      (CallFunction|Die))))

(fn ConstructionScript)

(fn TakeDamage
  (params (Damage :type Float%20%28double-precision%29))
  (if (> (- (Variables|Default|GetmaxLife) Damage) 0.0)
    (Variables|Default|SetmaxLife (- (Variables|Default|GetmaxLife) Damage))
    (else
      (Variables|Default|SetmaxLife 0.0))))
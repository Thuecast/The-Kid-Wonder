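; GolemShot_BP is a projectile for the Golem enemy, configured by a ShotType struct that sets its sprite, behavior, speed and damage.
; Each tick it moves along ShotDirection without sweep; the Following type first re-aims the direction and flipbook rotation at the player, while Lineal keeps its heading.
; On any actor overlap it damages LukeCharacter_BP if that is the other actor, then destroys itself, and it also expires after LifeTime.
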(event EventBeginPlay
  (Sprite|SetFlipbook (Variables|Default|GetShotFB) (.shotsprite (Variables|Default|GetshotType)))
  (Actor|SetLifeSpan (Variables|Default|GetlifeTime)))

(event Collision|EventActorBeginOverlap
  (params (OtherActor :type Actor%20Object%20Reference))
  (Utilities|FlowControl|Sequence
    (:then_0
      (bind _asluke_character_bp (Utilities|Casting|CastToLukeCharacter_BP OtherActor))
      (Game|Damage|ApplyDamage _asluke_character_bp (.shotdamage (Variables|Default|GetshotType)) 0 0))
    (:then_1
      (Actor|DestroyActor))))

(event EventTick
  (params (DeltaSeconds :type Float%20%28single-precision%29))
  (switch Utilities|FlowControl|Switch|SwitchonTypeOfShot (.shottype (Variables|Default|GetshotType))
    (:NewEnumerator0
      (CallFunction|ShotMovement))
    (:NewEnumerator1
      (CallFunction|SetDirectionandRotation)
      (CallFunction|ShotMovement))))

(fn ConstructionScript)

(fn ShotMovement
  (Transformation|SetActorLocation (+ (* (* (Utilities|Time|GetWorldDeltaSeconds) (.shotspeed (Variables|Default|GetshotType))) (Variables|Default|GetShotDirection)) (Transformation|GetActorLocation)) false false))

(fn SetDirectionandRotation
  (bind _returnvalue (Game|GetPlayerCharacter 0))
  (Variables|Default|SetShotDirection (Math|Vector|GetUnitDirection(Vector) (Transformation|GetActorLocation) (Transformation|GetActorLocation _returnvalue)))
  (Transformation|SetRelativeRotation (Variables|Default|GetShotFB) (Math|Rotator|FindLookatRotation (Transformation|GetActorLocation) (Transformation|GetActorLocation _returnvalue)) false false))
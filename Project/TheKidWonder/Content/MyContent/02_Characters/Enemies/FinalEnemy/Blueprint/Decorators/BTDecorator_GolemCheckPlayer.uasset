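; Behavior tree decorator that checks whether the Golem enemy can detect and see the Luke player character.
; A zero-length sphere trace around the Golem's capsule looks for Luke within the detection radius, then CheckVision line-traces to him to confirm line of sight.
; A confirmed sighting sets the IsSeeing blackboard key and passes the condition.
; A failed sphere check clears the key, but a blocked line trace fails without clearing it.
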(fn PerformConditionCheckAI
  (params (OwnerController :type AI%20Controller%20Object%20Reference) (ControlledPawn :type Pawn%20Object%20Reference))
  (bind _asgolem_bp (Utilities|Casting|CastToGolem_BP ControlledPawn))
  (bind (_outhit _returnvalue) (Collision|SphereTraceByChannel (Transformation|GetWorldLocation (Variables|/Script/Engine.Character|GetCapsuleComponent _asgolem_bp)) (Transformation|GetWorldLocation (Variables|/Script/Engine.Character|GetCapsuleComponent _asgolem_bp)) (Variables|Default|GetRadiusDetection) "TraceTypeQuery3" false 0 "None"))
  (if _returnvalue
    (bind _asluke_character_bp (Utilities|Casting|CastToLukeCharacter_BP (.HitActor (Collision|BreakHitResult _outhit)))
      (:then
        (bind _detected (CallFunction|CheckVision _asluke_character_bp _asgolem_bp))
        (return _detected))
      (:CastFailed
        _)))
  (Class|BTFunctionLibrary|SetBlackboardValueasBool (Variables|Default|GetisSeeing) false)
  (return false))

(fn CheckVision
  (params (TargetPlayer :type Luke%20Character%20BP%20Object%20Reference) (Himself :type Paper%20Character%20Object%20Reference))
  (Utilities|IsValid TargetPlayer
    (:Is%20Valid
      (bind _outhit (Collision|LineTraceByChannel (Transformation|GetWorldLocation (Variables|/Script/Engine.Character|GetCapsuleComponent Himself)) (Transformation|GetActorLocation TargetPlayer) "TraceTypeQuery3" false 0 "None"))
      (Utilities|Casting|CastToLukeCharacter_BP (.HitActor (Collision|BreakHitResult _outhit))
        (:then
          (Class|BTFunctionLibrary|SetBlackboardValueasBool (Variables|Default|GetisSeeing) true)
          (return true))
        (:CastFailed
          (return false))))))
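; Behavior tree decorator for the final enemy that checks whether the golem has run out of life.
; It casts the controlled pawn to Golem_BP and passes when GolemLife is zero or below, failing otherwise or if the cast fails.
; As a side effect, the condition check writes the result to the IsDead blackboard key whenever the cast succeeds.
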(fn PerformConditionCheckAI
  (params (OwnerController :type AI%20Controller%20Object%20Reference) (ControlledPawn :type Pawn%20Object%20Reference))
  (bind _asgolem_bp (Utilities|Casting|CastToGolem_BP ControlledPawn)
    (:then
      (if (<= (Variables|/Game/MyContent/02_Characters/Enemies/FinalEnemy/Blueprint/Golem_BP.Golem_BP_C|GetGolemLife _asgolem_bp) 0.0)
        (Class|BTFunctionLibrary|SetBlackboardValueasBool (Variables|Default|GetisDead) true)
        (return true)
        (else
          (Class|BTFunctionLibrary|SetBlackboardValueasBool (Variables|Default|GetisDead) false)
          (return false))))
    (:CastFailed
      (return false))))
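; Final-enemy Golem with flipbook animation, whose death brings up the win screen and pauses the game.
; It hands itself to its life bar widget, and unblocked damage lowers its life, with a one-time hit animation and sound.
; At zero life it plays its death animation, disables collision and destroys itself after a delay.
; GolemShoot spawns a typed projectile, offsetting the spawn point according to the player's side.
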(event Custom|Death
  (bind _sprite (Variables|Default|GetSprite))
  ;[1 1 1] Hit & Death
  (Variables|Default|SetGolemLife 0.0)
  (Sprite|SetFlipbook _sprite "/Game/MyContent/02_Characters/Enemies/FinalEnemy/FB/Golem_Death_FB.Golem_Death_FB")
  (Components|Timeline|SetLooping _sprite false)
  (Collision|SetCollisionEnabled (Variables|Collision|GetCapsuleComponent) "NoCollision")
  (Utilities|FlowControl|Delay 3.0)
  (Actor|DestroyActor)
  (Audio|PlaySoundatLocation "/Game/MyContent/04_SFX/Battle_SFX/69_Enemy_death_01.69_Enemy_death_01" (Transformation|GetActorLocation) "0, 0, 0" 1.0 1.0 0.0 0 0 0 0)
  (bind _returnvalue (UserInterface|CreateWidget "/Game/MyContent/03_UserInterface/YouWin_WB.YouWin_WB_C" (Game|GetPlayerController 0)))
  (UserInterface|Viewport|AddtoViewport _returnvalue 0)
  (Game|SetGamePaused true))

(event EventBeginPlay
  (bind _asgolem_life_bar_wb (Utilities|Casting|CastToGolem_LifeBar_WB (UserInterface|GetWidget (Variables|Default|GetLifebar))))
  (Variables|/Game/MyContent/02_Characters/Enemies/FinalEnemy/Blueprint/Golem_LifeBar_WB.Golem_LifeBar_WB_C|SetGolemRef _asgolem_life_bar_wb self))

(event Collision|EventActorBeginOverlap
  (params (OtherActor :type Actor%20Object%20Reference)))

(event EventTick
  (params (DeltaSeconds :type Float%20%28single-precision%29)))

(event Game|Damage|EventAnyDamage
  (params (Damage :type Float%20%28single-precision%29) (DamageType :type Damage%20Type%20Object%20Reference) (InstigatedBy :type Controller%20Object%20Reference) (DamageCauser :type Actor%20Object%20Reference))
  ;[1 1 1] Hit & Death
  (if (not (Variables|Default|GetisBlocking))
    (if (> (Math|Float|Clamp(Float) (- (Variables|Default|GetGolemLife) Damage) 0.0 (Variables|Default|GetGolemMaxLife)) 0.0)
      (Variables|Default|SetGolemLife (Math|Float|Clamp(Float) (- (Variables|Default|GetGolemLife) Damage) 0.0 (Variables|Default|GetGolemMaxLife)))
      (Utilities|FlowControl|DoOnce false
        (:Completed
          (Sprite|SetFlipbook (Variables|Default|GetSprite) "/Game/MyContent/02_Characters/Enemies/FinalEnemy/FB/Golem_Hit_FB.Golem_Hit_FB")
          (Audio|PlaySoundatLocation "/Game/MyContent/04_SFX/Player_Movement_SFX/61_Hit_03.61_Hit_03" (Transformation|GetActorLocation) "0, 0, 0" 1.0 1.0 0.0 0 0 0 0)))
      (else
        (CallFunction|Death)))))

(fn ConstructionScript)

(fn GolemShoot
  (bind _shotpoint (Variables|Default|GetShotPoint))
  (bind _sprite (Variables|Default|GetSprite))
  (bind _returnvalue (Transformation|GetWorldLocation _shotpoint))
  (if (< (.x (Transformation|GetWorldLocation (Variables|Default|GetSprite))) (.x (Transformation|GetActorLocation (Game|GetPlayerCharacter 0))))
    (bind _returnvalue_2 (Game|SpawnActorfromClass "/Game/MyContent/02_Characters/Enemies/FinalEnemy/Blueprint/GolemShot_BP.GolemShot_BP_C" (Math|Transform|MakeTransform (Transformation|GetWorldLocation (Variables|Default|GetShotPoint)) "0, 0, 0" "1.000000,1.000000,1.000000") "AlwaysSpawn" "MultiplyWithRoot" 0 (Variables|Default|GetshotType) 0))
    (Default|SetDirectionandRotation _returnvalue_2)
    (else
      (bind _returnvalue_3 (Game|SpawnActorfromClass "/Game/MyContent/02_Characters/Enemies/FinalEnemy/Blueprint/GolemShot_BP.GolemShot_BP_C" (Math|Transform|MakeTransform (Math|Vector|MakeVector (- (.x _returnvalue) 8e+01) (.y _returnvalue) (.z _returnvalue)) "0, 0, 0" "1.000000,1.000000,1.000000") "AlwaysSpawn" "MultiplyWithRoot" 0 (Variables|Default|GetshotType) 0))
      (Default|SetDirectionandRotation _returnvalue_3)))
  (Sprite|SetFlipbook _sprite "/Game/MyContent/02_Characters/Enemies/FinalEnemy/FB/Golem_FistShot_FB.Golem_FistShot_FB")
  (Components|Timeline|SetLooping _sprite true)
  (Audio|Components|Audio|Play _sprite))
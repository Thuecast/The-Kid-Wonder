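; Behavior tree task that steps the Golem enemy along the X axis toward the player in a 2D Paper2D setup.
; Each execution sets the idle flipbook, compares X positions, then calls MoveLeft or MoveRight.
; These offset the actor's location by speed and delta time and mirror the sprite through its X scale.
; The task succeeds after one step, failing only if the pawn is not a Golem_BP.
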(event EventReceiveExecuteAI
  (params (OwnerController :type AI%20Controller%20Object%20Reference) (ControlledPawn :type Pawn%20Object%20Reference))
  (bind _asgolem_bp (Utilities|Casting|CastToGolem_BP ControlledPawn)
    (:then
      (Sprite|SetFlipbook (Variables|/Script/Paper2D.PaperCharacter|GetSprite _asgolem_bp) "/Game/MyContent/02_Characters/Enemies/FinalEnemy/FB/Golem_Idle_FB.Golem_Idle_FB")
      (bind _isright (CallFunction|CheckDirectiontoPlayer _asgolem_bp))
      (if _isright
        (CallFunction|MoveLeft _asgolem_bp)
        (else
          (CallFunction|MoveRight _asgolem_bp)))
      (AI|BehaviorTree|FinishExecute true))
    (:CastFailed
      (AI|BehaviorTree|FinishExecute false))))

(fn CheckDirectiontoPlayer
  (params (himself :type Golem%20BP%20Object%20Reference))
  (return (>= (- (.x (Transformation|GetActorLocation himself)) (.x (Transformation|GetActorLocation (Game|GetPlayerCharacter 0)))) 0.0)))

(fn MoveRight
  (params (himself :type Golem%20BP%20Object%20Reference))
  (bind _returnvalue (Transformation|GetActorLocation himself))
  (bind _output_get (Variables|/Game/MyContent/02_Characters/Enemies/FinalEnemy/Blueprint/Golem_BP.Golem_BP_C|SetGolemDirection himself 1.0))
  (Transformation|SetActorLocation himself (Math|Vector|MakeVector (+ (* (Utilities|Time|GetWorldDeltaSeconds) (Variables|/Game/MyContent/02_Characters/Enemies/FinalEnemy/Blueprint/Golem_BP.Golem_BP_C|GetGolemSpeed himself) (Variables|/Game/MyContent/02_Characters/Enemies/FinalEnemy/Blueprint/Golem_BP.Golem_BP_C|GetGolemDirection himself)) (.x _returnvalue)) (.y _returnvalue) (.z _returnvalue)) false false)
  (Transformation|SetRelativeScale3D (Variables|/Script/Paper2D.PaperCharacter|GetSprite himself) (Math|Vector|MakeVector _output_get 1.0 1.0)))

(fn MoveLeft
  (params (himself :type Golem%20BP%20Object%20Reference))
  (bind _returnvalue (Transformation|GetActorLocation himself))
  (bind _output_get (Variables|/Game/MyContent/02_Characters/Enemies/FinalEnemy/Blueprint/Golem_BP.Golem_BP_C|SetGolemDirection himself -1.0))
  (Transformation|SetActorLocation himself (Math|Vector|MakeVector (+ (* (Utilities|Time|GetWorldDeltaSeconds) (Variables|/Game/MyContent/02_Characters/Enemies/FinalEnemy/Blueprint/Golem_BP.Golem_BP_C|GetGolemSpeed himself) (Variables|/Game/MyContent/02_Characters/Enemies/FinalEnemy/Blueprint/Golem_BP.Golem_BP_C|GetGolemDirection himself)) (.x _returnvalue)) (.y _returnvalue) (.z _returnvalue)) false false)
  (Transformation|SetRelativeScale3D (Variables|/Script/Paper2D.PaperCharacter|GetSprite himself) (Math|Vector|MakeVector _output_get 1.0 1.0)))
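; Behavior tree decorator that decides whether the Golem final enemy can attack the player.
; It runs a zero-length sphere trace of RadiusAttack around the Golem's capsule and passes only if the hit actor is LukeCharacter_BP.
; It also writes that character to the Player blackboard key, or sets the key to none when the check fails.
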(fn PerformConditionCheckAI
  (params (OwnerController :type AI%20Controller%20Object%20Reference) (ControlledPawn :type Pawn%20Object%20Reference))
  (bind _player (Variables|Default|GetPlayer))
  (bind _asgolem_bp (Utilities|Casting|CastToGolem_BP ControlledPawn))
  (bind (_outhit _returnvalue) (Collision|SphereTraceByChannel (Transformation|GetWorldLocation (Variables|/Script/Engine.Character|GetCapsuleComponent _asgolem_bp)) (Transformation|GetWorldLocation (Variables|/Script/Engine.Character|GetCapsuleComponent _asgolem_bp)) (Variables|Default|GetRadiusAttack) "TraceTypeQuery3" false 0 "None"))
  (if _returnvalue
    (bind _asluke_character_bp (Utilities|Casting|CastToLukeCharacter_BP (.HitActor (Collision|BreakHitResult _outhit)))
      (:then
        (Class|BTFunctionLibrary|SetBlackboardValueasObject _player _asluke_character_bp)
        (return true))
      (:CastFailed
        _)))
  (Class|BTFunctionLibrary|SetBlackboardValueasObject _player)
  (return false))
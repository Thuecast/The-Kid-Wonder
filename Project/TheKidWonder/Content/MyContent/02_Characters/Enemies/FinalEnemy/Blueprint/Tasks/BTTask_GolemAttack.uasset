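; Behavior tree task that makes the Golem enemy fire one of two randomly chosen ranged attacks, a fist shot or a head shot.
; It plays the matching looping flipbook, waits briefly, spawns a GolemShot_BP of that type at the shot or head point, then finishes.
; Each shot function compares Golem and player X positions, shifting the spawn point when the player is not to the right, then has the projectile set its direction and rotation.
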(event EventReceiveExecuteAI
  (params (OwnerController :type AI%20Controller%20Object%20Reference) (ControlledPawn :type Pawn%20Object%20Reference))
  (bind _asgolem_bp (Utilities|Casting|CastToGolem_BP ControlledPawn)
    (:then
      (bind _output_get (Variables|Default|SetOption (Math|Random|RandomIntegerinRange 0 1)))
      (if (== _output_get 0)
        (Sprite|SetFlipbook (Variables|/Script/Paper2D.PaperCharacter|GetSprite _asgolem_bp) "/Game/MyContent/02_Characters/Enemies/FinalEnemy/FB/Golem_FistShot_FB.Golem_FistShot_FB")
        (Components|Timeline|SetLooping (Variables|/Script/Paper2D.PaperCharacter|GetSprite _asgolem_bp) true)
        (Audio|Components|Audio|Play (Variables|/Script/Paper2D.PaperCharacter|GetSprite _asgolem_bp))
        (Utilities|FlowControl|Delay 0.5)
        (CallFunction|FistShot _asgolem_bp)
        (else
          (Sprite|SetFlipbook (Variables|/Script/Paper2D.PaperCharacter|GetSprite _asgolem_bp) "/Game/MyContent/02_Characters/Enemies/FinalEnemy/FB/Golem_HeadShot_FB.Golem_HeadShot_FB")
          (Components|Timeline|SetLooping (Variables|/Script/Paper2D.PaperCharacter|GetSprite _asgolem_bp) true)
          (Audio|Components|Audio|Play (Variables|/Script/Paper2D.PaperCharacter|GetSprite _asgolem_bp))
          (Utilities|FlowControl|Delay 0.5)
          (CallFunction|HeadShot _asgolem_bp)))
      (AI|BehaviorTree|FinishExecute true))
    (:CastFailed
      (AI|BehaviorTree|FinishExecute false))))

(fn FistShot
  (params (himself :type Golem%20BP%20Object%20Reference))
  (bind _shotpoint (Variables|/Game/MyContent/02_Characters/Enemies/FinalEnemy/Blueprint/Golem_BP.Golem_BP_C|GetShotPoint himself))
  (bind _returnvalue (Transformation|GetWorldLocation _shotpoint))
  (if (< (.x (Transformation|GetWorldLocation (Variables|/Script/Paper2D.PaperCharacter|GetSprite himself))) (.x (Transformation|GetActorLocation (Game|GetPlayerCharacter 0))))
    (bind _returnvalue_2 (Game|SpawnActorfromClass "/Game/MyContent/02_Characters/Enemies/FinalEnemy/Blueprint/GolemShot_BP.GolemShot_BP_C" (Math|Transform|MakeTransform (Transformation|GetWorldLocation _shotpoint) "0, 0, 0" "1.000000,1.000000,1.000000") "AlwaysSpawn" "MultiplyWithRoot" 0 (Variables|Default|GetFistType) 0))
    (Default|SetDirectionandRotation _returnvalue_2)
    (else
      (bind _returnvalue_3 (Game|SpawnActorfromClass "/Game/MyContent/02_Characters/Enemies/FinalEnemy/Blueprint/GolemShot_BP.GolemShot_BP_C" (Math|Transform|MakeTransform (Math|Vector|MakeVector (- (.x _returnvalue) 6e+01) (.y _returnvalue) (.z _returnvalue)) "0, 0, 0" "1.000000,1.000000,1.000000") "AlwaysSpawn" "MultiplyWithRoot" 0 (Variables|Default|GetFistType) 0))
      (Default|SetDirectionandRotation _returnvalue_3)))
  (return))

(fn HeadShot
  (params (himself :type Golem%20BP%20Object%20Reference))
  (bind _headpoint (Variables|/Game/MyContent/02_Characters/Enemies/FinalEnemy/Blueprint/Golem_BP.Golem_BP_C|GetHeadPoint himself))
  (bind _returnvalue (Transformation|GetWorldLocation _headpoint))
  (if (< (.x (Transformation|GetWorldLocation (Variables|/Script/Paper2D.PaperCharacter|GetSprite himself))) (.x (Transformation|GetActorLocation (Game|GetPlayerCharacter 0))))
    (bind _returnvalue_2 (Game|SpawnActorfromClass "/Game/MyContent/02_Characters/Enemies/FinalEnemy/Blueprint/GolemShot_BP.GolemShot_BP_C" (Math|Transform|MakeTransform (Transformation|GetWorldLocation _headpoint) "0, 0, 0" "1.000000,1.000000,1.000000") "AlwaysSpawn" "MultiplyWithRoot" 0 (Variables|Default|GetHeadType) 0))
    (Default|SetDirectionandRotation _returnvalue_2)
    (else
      (bind _returnvalue_3 (Game|SpawnActorfromClass "/Game/MyContent/02_Characters/Enemies/FinalEnemy/Blueprint/GolemShot_BP.GolemShot_BP_C" (Math|Transform|MakeTransform (Math|Vector|MakeVector (- (.x _returnvalue) 4.0) (.y _returnvalue) (.z _returnvalue)) "0, 0, 0" "1.000000,1.000000,1.000000") "AlwaysSpawn" "MultiplyWithRoot" 0 (Variables|Default|GetHeadType) 0))
      (Default|SetDirectionandRotation _returnvalue_3)))
  (return))
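; Behavior tree task that makes the Golem enemy fire a projectile from its head.
; It switches the Paper2D sprite to a looping head-shot flipbook, waits briefly, then spawns a shot actor at the HeadPoint with the task's ShotType.
; The player's X position relative to the sprite picks the branch, with one side nudging the spawn X slightly, and each shot then sets its direction and rotation.
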(event EventReceiveExecuteAI
  (params (OwnerController :type AI%20Controller%20Object%20Reference) (ControlledPawn :type Pawn%20Object%20Reference))
  (bind _asgolem_bp (Utilities|Casting|CastToGolem_BP ControlledPawn)
    (:then
      (Sprite|SetFlipbook (Variables|/Script/Paper2D.PaperCharacter|GetSprite _asgolem_bp) "/Game/MyContent/02_Characters/Enemies/FinalEnemy/FB/Golem_HeadShot_FB.Golem_HeadShot_FB")
      (Components|Timeline|SetLooping (Variables|/Script/Paper2D.PaperCharacter|GetSprite _asgolem_bp) true)
      (Audio|Components|Audio|Play (Variables|/Script/Paper2D.PaperCharacter|GetSprite _asgolem_bp))
      (Utilities|FlowControl|Delay 0.5)
      (if (< (.x (Transformation|GetWorldLocation (Variables|/Script/Paper2D.PaperCharacter|GetSprite _asgolem_bp))) (.x (Transformation|GetActorLocation (Game|GetPlayerCharacter 0))))
        (bind _returnvalue (Game|SpawnActorfromClass "/Game/MyContent/02_Characters/Enemies/FinalEnemy/Blueprint/GolemShot_BP.GolemShot_BP_C" (Math|Transform|MakeTransform (Transformation|GetWorldLocation (Variables|/Game/MyContent/02_Characters/Enemies/FinalEnemy/Blueprint/Golem_BP.Golem_BP_C|GetHeadPoint _asgolem_bp)) "0, 0, 0" "1.000000,1.000000,1.000000") "AlwaysSpawn" "MultiplyWithRoot" 0 (Variables|Default|GetshotType) 0))
        (Default|SetDirectionandRotation _returnvalue)
        (else
          (bind _returnvalue_2 (Game|SpawnActorfromClass "/Game/MyContent/02_Characters/Enemies/FinalEnemy/Blueprint/GolemShot_BP.GolemShot_BP_C" (Math|Transform|MakeTransform (Math|Vector|MakeVector (- (.x (Transformation|GetWorldLocation (Variables|/Game/MyContent/02_Characters/Enemies/FinalEnemy/Blueprint/Golem_BP.Golem_BP_C|GetHeadPoint _asgolem_bp))) 4.0) (.y (Transformation|GetWorldLocation (Variables|/Game/MyContent/02_Characters/Enemies/FinalEnemy/Blueprint/Golem_BP.Golem_BP_C|GetHeadPoint _asgolem_bp))) (.z (Transformation|GetWorldLocation (Variables|/Game/MyContent/02_Characters/Enemies/FinalEnemy/Blueprint/Golem_BP.Golem_BP_C|GetHeadPoint _asgolem_bp)))) "0, 0, 0" "1.000000,1.000000,1.000000") "AlwaysSpawn" "MultiplyWithRoot" 0 (Variables|Default|GetshotType) 0))
          (Default|SetDirectionandRotation _returnvalue_2)))
      (AI|BehaviorTree|FinishExecute true))
    (:CastFailed
      (AI|BehaviorTree|FinishExecute false))))